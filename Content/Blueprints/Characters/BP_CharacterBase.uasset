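; Base character Blueprint that handles weapons, interaction and incoming damage.
; Weapons spawn by DT_WeaponStats type onto WeaponScene; switching cycles backpack keys, toggling instances cached in MapOfWeapons or spawning missing ones.
; InteractSphere tracks an interface-implementing actor for ActionUse, while AnyDamage forwards BP_DamageObject damage to BPMainStatsComponent.
; UpdateWeaponSceneRotation runs on Tick but is empty here, and SpawnWeapon_0/_1 are uncalled, partial copies of SpawnWeapon.
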(event OnComponentBeginOverlap(InteractSphere)
  (params (OverlappedComponent :type Primitive%20Component%20Object%20Reference) (OtherActor :type Actor%20Object%20Reference) (OtherComp :type Primitive%20Component%20Object%20Reference) (OtherBodyIndex :type Integer) (bFromSweep :type Boolean) (SweepResult :type Hit%20Result%20Structure%20%28by%20ref%29))
  (if (Utilities|DoesObjectImplementInterface OtherActor "/Game/Blueprints/BPI_CustomInterface.BPI_CustomInterface_C")
    (Variables|Default|SetActorToInteract OtherActor)))

(event OnComponentEndOverlap(InteractSphere)
  (params (OverlappedComponent :type Primitive%20Component%20Object%20Reference) (OtherActor :type Actor%20Object%20Reference) (OtherComp :type Primitive%20Component%20Object%20Reference) (OtherBodyIndex :type Integer))
  (Variables|Default|SetActorToInteract 0))

(event EventBeginPlay
  (Weapon|UpdateCurrentWeapon "None"))

(event Collision|EventActorBeginOverlap
  (params (OtherActor :type Actor%20Object%20Reference)))

(event EventTick
  (params (DeltaSeconds :type Float%20%28single-precision%29))
  (Weapon|UpdateWeaponSceneRotation))

(event Game|Damage|EventAnyDamage
  (params (Damage :type Float%20%28single-precision%29) (DamageType :type Damage%20Type%20Object%20Reference) (InstigatedBy :type Controller%20Object%20Reference) (DamageCauser :type Actor%20Object%20Reference))
  (bind _asbp_damage_object (Utilities|Casting|CastToBP_DamageObject DamageType))
  (Default|ReceiveDamage (Variables|Default|GetBP_MainStatsComponent) Damage (Variables|/Game/Blueprints/Objects/BP_DamageObject.BP_DamageObject_C|GetDamageType _asbp_damage_object) DamageCauser))

(fn ConstructionScript)

(fn ActionUse
  (bind _actortointeract (Variables|Default|GetActorToInteract)
    (:then
      (Class|BPICustomInterface|Interacts(Message) _actortointeract))
    (:else)))

(fn ActionMain
  (params (IsPressed :type Boolean))
  (Variables|Default|SetIsActionMainPressed IsPressed)
  (bind _currentweapon (Variables|Default|GetCurrentWeapon)
    (:then
      (Default|ShootingProcess _currentweapon (Variables|Default|GetIsActionMainPressed)))
    (:else)))

(fn UpdateCurrentWeapon
  (params (InWeaponName :type Name))
  (Utilities|FlowControl|Sequence
    (:then_0
      (if (Utilities|Name|NotEqual(Name) InWeaponName "None")
        (LocalVariables|SetL_Name InWeaponName)
        (elif (> (Utilities|Map|Length (Variables|/Game/Blueprints/Components/BP_BackpackComponent.BP_BackpackComponent_C|GetAvalableWeapon (Variables|Default|GetBP_BackpackComponent))) 0)
          (bind _keys (Utilities|Map|Keys (Variables|/Game/Blueprints/Components/BP_BackpackComponent.BP_BackpackComponent_C|GetAvalableWeapon (Variables|Default|GetBP_BackpackComponent))))
          (LocalVariables|SetL_Name (Utilities|Array|Get(acopy) _keys)))))
    (:then_1
      (bind _returnvalue (Utilities|GetDataTableRow "/Game/Data/DT_WeaponStats.DT_WeaponStats" (LocalVariables|GetL_Name))
        (:then
          (LocalVariables|SetL_Row _returnvalue)
          (Utilities|FlowControl|Sequence
            (:then_0
              (bind _currentweapon (Variables|Default|GetCurrentWeapon)
                (:then
                  (Default|ActivateWeapon _currentweapon false)
                  (Variables|Default|SetCurrentWeapon 0))
                (:else)))
            (:then_1
              (Weapon|SpawnWeapon (LocalVariables|GetL_Name) (Utilities|Struct|BreakSTRUCT_WeaponStats (LocalVariables|GetL_Row))))))))))

(fn SpawnWeapon
  (params (InWeaponName :type Name) (InWeaponType :type ENUM_WeaponType%20Enum :default "NewEnumerator0"))
  (if (Utilities|Name|NotEqual(Name) InWeaponName "None")
    (if (not (Utilities|IsValid (Variables|Default|GetCurrentWeapon)))
      (bind _returnvalue (Game|SpawnActorfromClass (Utilities|Select :Index InWeaponType :NewEnumerator0 "/Game/Blueprints/Weapons/BP_Weapon_Pistol.BP_Weapon_Pistol_C" :NewEnumerator1 "/Game/Blueprints/Weapons/BP_Weapon_Rifle.BP_Weapon_Rifle_C" :NewEnumerator2 "/Game/Blueprints/Weapons/BP_Weapon_ShotGun.BP_Weapon_ShotGun_C" :NewEnumerator3 "/Game/Blueprints/Weapons/BP_Weapon_RocketLauncher.BP_Weapon_RocketLauncher_C" :NewEnumerator4 "/Game/Blueprints/Weapons/BP_Weapon_SniperRifle.BP_Weapon_SniperRifle_C") (Transformation|GetWorldTransform (Variables|Default|GetWeaponScene)) "Undefined" self 0))
      (bind _asbp_weapon_base (Utilities|Casting|CastToBP_WeaponBase _returnvalue))
      (Variables|Default|SetCurrentWeapon _asbp_weapon_base)
      (Transformation|AttachComponentToComponent (Variables|Default|GetCurrentWeapon) (Variables|Default|GetWeaponScene) "None" "SnapToTarget" "SnapToTarget" "KeepRelative" true)
      (Default|ConfiigureWeaponStats (Variables|Default|GetCurrentWeapon) InWeaponName)
      (Variables|Default|SetCurrentWeaponName InWeaponName)
      (Utilities|Map|Add (Variables|Default|GetMapOfWeapons) InWeaponName (Variables|Default|GetCurrentWeapon))
      (Default|CallOnWeaponChanged))))

(fn SwitchWeapon
  (params (InNextWeapon :type Boolean))
  (Variables|Default|GetCurrentWeapon
    (:then
      (Weapon|GetNextWeapon InNextWeapon)
      (bind _returnvalue (Utilities|GetDataTableRow "/Game/Data/DT_WeaponStats.DT_WeaponStats" (Variables|Default|GetCurrentWeaponName))
        (:then
          (Weapon|SpawnWeapon (Variables|Default|GetCurrentWeaponName) (.WeaponType (Utilities|Struct|BreakSTRUCT_WeaponStats _returnvalue))))))
    (:else)))

(fn GetNextWeapon
  (params (InNextWepon :type Boolean))
  (bind _keys (Utilities|Map|Keys (Variables|/Game/Blueprints/Components/BP_BackpackComponent.BP_BackpackComponent_C|GetAvalableWeapon (Variables|Default|GetBP_BackpackComponent))))
  (LocalVariables|SetL_AvalableWeaponNames _keys)
  (LocalVariables|SetL_CurrentIndex (Utilities|Array|FindItem (LocalVariables|GetL_AvalableWeaponNames) (Variables|Default|GetCurrentWeaponName)))
  (Utilities|FlowControl|Sequence
    (:then_0
      (if (.ReturnValue (Utilities|Map|Find (Variables|Default|GetMapOfWeapons) (Variables|Default|GetCurrentWeaponName)))
        (Default|ActivateWeapon (.Value (Utilities|Map|Find (Variables|Default|GetMapOfWeapons) (Variables|Default|GetCurrentWeaponName))) false)
        (Variables|Default|SetCurrentWeapon 0)))
    (:then_1
      (if InNextWepon
        (Math|Integer|IncrementInt (LocalVariables|GetL_CurrentIndex)
          (:%20%20
            (if (<= (LocalVariables|GetL_CurrentIndex) (Utilities|Array|LastIndex (LocalVariables|GetL_AvalableWeaponNames)))
              (Variables|Default|SetCurrentWeaponName (Utilities|Array|Get(acopy) (LocalVariables|GetL_AvalableWeaponNames) (LocalVariables|GetL_CurrentIndex)))
              (else
                (Variables|Default|SetCurrentWeaponName (Utilities|Array|Get(acopy) (LocalVariables|GetL_AvalableWeaponNames)))))))
        (else
          (Math|Integer|DecrementInt (LocalVariables|GetL_CurrentIndex)
            (:%20%20
              (if (< (LocalVariables|GetL_CurrentIndex) 0)
                (Variables|Default|SetCurrentWeaponName (Utilities|Array|Get(acopy) (LocalVariables|GetL_AvalableWeaponNames) (Utilities|Array|LastIndex (LocalVariables|GetL_AvalableWeaponNames))))
                (else
                  (Variables|Default|SetCurrentWeaponName (Utilities|Array|Get(acopy) (LocalVariables|GetL_AvalableWeaponNames) (LocalVariables|GetL_CurrentIndex))))))))))
    (:then_2
      (if (.ReturnValue (Utilities|Map|Find (Variables|Default|GetMapOfWeapons) (Variables|Default|GetCurrentWeaponName)))
        (Default|ActivateWeapon (.Value (Utilities|Map|Find (Variables|Default|GetMapOfWeapons) (Variables|Default|GetCurrentWeaponName))) true)
        (Variables|Default|SetCurrentWeapon (.Value (Utilities|Map|Find (Variables|Default|GetMapOfWeapons) (Variables|Default|GetCurrentWeaponName))))
        (else
          (Variables|Default|SetCurrentWeapon 0))))
    (:then_3
      (Default|CallOnWeaponChanged))))

(fn ReloadWeapon
  (Variables|Default|GetCurrentWeapon
    (:then
      (Default|Reaload (Variables|Default|GetCurrentWeapon)))
    (:else)))

(fn UpdateWeaponSceneRotation)

(fn SpawnWeapon0
  (params (InWeaponName :type Name) (InWeaponType :type ENUM_WeaponType%20Enum :default "NewEnumerator0"))
  (if (Utilities|Name|NotEqual(Name) InWeaponName "None")
    (if (not (Utilities|IsValid (Variables|Default|GetCurrentWeapon)))
      (bind _returnvalue (Game|SpawnActorfromClass (Utilities|Select :Index InWeaponType :NewEnumerator0 "/Game/Blueprints/Weapons/BP_Weapon_Pistol.BP_Weapon_Pistol_C" :NewEnumerator1 "/Game/Blueprints/Weapons/BP_Weapon_Rifle.BP_Weapon_Rifle_C" :NewEnumerator2 0 :NewEnumerator3 0 :NewEnumerator4 0) (Transformation|GetWorldTransform (Variables|Default|GetWeaponScene)) "Undefined" self 0))
      (bind _asbp_weapon_base (Utilities|Casting|CastToBP_WeaponBase _returnvalue))
      (Variables|Default|SetCurrentWeapon _asbp_weapon_base)
      (Transformation|AttachComponentToComponent (Variables|Default|GetCurrentWeapon) (Variables|Default|GetWeaponScene) "None" "SnapToTarget" "SnapToTarget" "KeepRelative" true)
      (Default|ConfiigureWeaponStats (Variables|Default|GetCurrentWeapon) InWeaponName)
      (Variables|Default|SetCurrentWeaponName InWeaponName)
      (Utilities|Map|Add (Variables|Default|GetMapOfWeapons) InWeaponName (Variables|Default|GetCurrentWeapon)))))

(fn SpawnWeapon1
  (params (InWeaponName :type Name) (InWeaponType :type ENUM_WeaponType%20Enum :default "NewEnumerator0"))
  (if (Utilities|Name|NotEqual(Name) InWeaponName "None")
    (if (not (Utilities|IsValid (Variables|Default|GetCurrentWeapon)))
      (bind _returnvalue (Game|SpawnActorfromClass (Utilities|Select :Index InWeaponType :NewEnumerator0 "/Game/Blueprints/Weapons/BP_Weapon_Pistol.BP_Weapon_Pistol_C" :NewEnumerator1 "/Game/Blueprints/Weapons/BP_Weapon_Rifle.BP_Weapon_Rifle_C" :NewEnumerator2 0 :NewEnumerator3 0 :NewEnumerator4 0) (Transformation|GetWorldTransform (Variables|Default|GetWeaponScene)) "Undefined" self 0))
      (bind _asbp_weapon_base (Utilities|Casting|CastToBP_WeaponBase _returnvalue))
      (Variables|Default|SetCurrentWeapon _asbp_weapon_base)
      (Transformation|AttachComponentToComponent (Variables|Default|GetCurrentWeapon) (Variables|Default|GetWeaponScene) "None" "SnapToTarget" "SnapToTarget" "KeepRelative" true)
      (Default|ConfiigureWeaponStats (Variables|Default|GetCurrentWeapon) InWeaponName)
      (Variables|Default|SetCurrentWeaponName InWeaponName)
      (Utilities|Map|Add (Variables|Default|GetMapOfWeapons) InWeaponName (Variables|Default|GetCurrentWeapon)))))