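; Blueprint function library with two general-purpose helper functions.
; CustomPrintString wraps PrintString, passing the world context, screen and log toggles, color and duration straight through.
; RNGVector scales each component of an input vector by its own random float within a given range and returns the results as separate X, Y and Z outputs.
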(fn CustomPrintString
  (params (WorldContextObject :type Object%20Object%20Reference) (InString :type String) (bPrintToScreen :type Boolean) (bPrintToLog :type Boolean) (TextColor :type Linear%20Color%20Structure :default "(R=0.500335,G=0.000000,B=0.562500,A=1.000000)") (Duration :type Float%20%28single-precision%29))
  (Development|PrintString WorldContextObject InString bPrintToScreen bPrintToLog TextColor Duration))

(fn RNGVector
  (params (InVector :type Vector) (InMin :type Float%20%28single-precision%29) (InMax :type Float%20%28single-precision%29))
  (return (Math|Vector|MakeVector (* (.x InVector) (Math|Random|RandomFloatinRange InMin InMax)) (* (.y InVector) (Math|Random|RandomFloatinRange InMin InMax)) (* (.z InVector) (Math|Random|RandomFloatinRange InMin InMax)))))