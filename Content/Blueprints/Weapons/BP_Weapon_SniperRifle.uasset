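; Sniper rifle weapon Blueprint that overrides the parent's single shot with a long-range hitscan line trace from the muzzle, with debug drawing left on.
; A hit pushes simulating components or fires a radial force, applies damage tripled on "head" bone hits, and spawns a randomly rolled, attached impact effect.
; Shot effects play on hit or miss, and the parent SingleShot is never called.
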(event EventBeginPlay
  (|CallParentFunction) ; This node is disabled and will not be called.\nDrag off pins to build functionality.
)

(event Collision|EventActorBeginOverlap
  (params (OtherActor :type Actor%20Object%20Reference))
  (|CallParentFunction OtherActor) ; This node is disabled and will not be called.\nDrag off pins to build functionality.
)

(event EventTick
  (params (DeltaSeconds :type Float%20%28single-precision%29))
  (|CallParentFunction DeltaSeconds) ; This node is disabled and will not be called.\nDrag off pins to build functionality.
)

(fn ConstructionScript
  (|CallParentFunction))

(fn ConfiigureWeaponStats
  (params (InWeaponName :type Name :default "None"))
  (|CallParentFunction InWeaponName)
  (Class|SkinnedMeshComponent|SetSkeletalMesh (Variables|Default|GetSkeletalMesh) 0 true))

(fn SingleShot
  (bind _muzzlescene (Variables|Default|GetMuzzleScene))
  (bind _returnvalue (Transformation|GetWorldLocation _muzzlescene))
  (Utilities|FlowControl|Sequence
    (:then_0
      (bind (_outhit _returnvalue_2) (Collision|LineTraceByChannel _returnvalue (+ _returnvalue (* (Math|Vector|GetForwardVector (Variables|Default|GetMuzzleScene)) 2.5e+04)) "TraceTypeQuery2" true (Utilities|Array|MakeArray self (Components|GetOwner)) "ForDuration" true "(R=1.000000,G=0.000000,B=0.000000,A=1.000000)" "(R=0.000000,G=1.000000,B=0.000000,A=1.000000)" 1e+01))
      (if _returnvalue_2
        (Variables|Default|SetHitResult _outhit)
        (Variables|Default|SetHitLocation (.Location (Collision|BreakHitResult (Variables|Default|GetHitResult))))
        (Variables|Default|SetHitNormal (.Normal (Collision|BreakHitResult (Variables|Default|GetHitResult))))
        (Variables|Default|SetHitActor (.HitActor (Collision|BreakHitResult (Variables|Default|GetHitResult))))
        (Variables|Default|SetHitComponent (.HitComponent (Collision|BreakHitResult (Variables|Default|GetHitResult))))
        (Utilities|FlowControl|Sequence
          (:then_0
            (Shoot|AddPhysicsImpulse))
          (:then_1
            (Shoot|ApplyDamagebyHitScan))
          (:then_2
            (Shoot|SpawnDecal)))))
    (:then_1
      (CallFunction|ShotEffects))))

(fn SpawnDecal
  (bind _hitnormal (Variables|Default|GetHitNormal))
  (bind _returnvalue (Math|Conversions|RotationFromXVector _hitnormal))
  (LocalVariables|SetL_Rotator (Math|Rotator|MakeRotator (Math|Random|RandomFloatinRange 0.0 3.6e+02) (.pitch _returnvalue) (.yaw _returnvalue)))
  (bind _returnvalue_2 (Game|SpawnActorfromClass "/Game/Blueprints/Weapons/Projectiles/BP_ImpactEffect.BP_ImpactEffect_C" (Math|Transform|MakeTransform (Variables|Default|GetHitLocation) (LocalVariables|GetL_Rotator) "1,1,1") "Undefined" self 0))
  (LocalVariables|SetL_Impact _returnvalue_2)
  (Transformation|AttachComponentToComponent (LocalVariables|GetL_Impact) (Variables|Default|GetOther) (.HitBoneName (Collision|BreakHitResult (Variables|Default|GetHitResult))) "KeepWorld" "KeepWorld" "KeepWorld" true))

(fn ApplyDamagebyHitScan
  (Utilities|FlowControl|Sequence
    (:then_0
      (LocalVariables|SetL_Damage (Variables|Default|GetDamageCurrent)))
    (:then_1
      (if (Utilities|Name|Equal(Name) (.HitBoneName (Collision|BreakHitResult (Variables|Default|GetHitResult))) "head")
        (LocalVariables|SetL_Damage (* (LocalVariables|GetL_Damage) 3))))
    (:then_2
      (Game|Damage|ApplyDamage (Variables|Default|GetHitActor) (Math|Conversions|ToFloat(Integer) (LocalVariables|GetL_Damage)) 0 (Components|GetOwner) "/Game/Blueprints/Objects/BP_DamageObject.BP_DamageObject_C"))))

(fn AddPhysicsImpulse
  (bind _hitcomponent (Variables|Default|GetHitComponent)
    (:then
      (if (Physics|IsSimulatingPhysics _hitcomponent "None")
        (Physics|AddImpulseatLocation (Variables|Default|GetHitComponent) (* (* (Math|Vector|Normalize (- (Variables|Default|GetHitLocation) (Transformation|GetWorldLocation (Variables|Default|GetMuzzleScene)))) 2e+03) (Variables|Default|GetImpulseMult)) (Variables|Default|GetHitLocation) "None")
        (else
          (Transformation|SetWorldLocation (Variables|Default|GetRadialForce) (Variables|Default|GetHitLocation) false false)
          (Class|RadialForceComponent|FireImpulse (Variables|Default|GetRadialForce)))))
    (:else)))