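; Missile projectile that boosts its speed after launch and spawns BP_Explosion on hit before destroying itself.
; BeginPlay and a one-shot 0.1-second timer each raise Acceleration by an exponent and add it to ProjectileMovement velocity along the travel direction, giving two boosts rather than continuous thrust.
; Empty overrides of OnEndOnHit, SpawnDecal and AddPhysicsImpulse suppress those parent behaviors.
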(event Custom|AddSpeed
  (Variables|Default|SetAcceleration (Math|Float|Power (Variables|Default|GetAcceleration) 1.2))
  (Variables|/Script/Engine.MovementComponent|SetVelocity (Variables|Default|GetProjectileMovement) (+ (* (Math|Vector|Normalize (Variables|/Script/Engine.MovementComponent|GetVelocity (Variables|Default|GetProjectileMovement))) (Variables|Default|GetAcceleration)) (Variables|/Script/Engine.MovementComponent|GetVelocity (Variables|Default|GetProjectileMovement)))))

(event EventBeginPlay
  (|CallParentFunction)
  (Utilities|Time|SetTimerbyEvent (delegate Custom|AddSpeed) 0.1)
  (Variables|Default|SetAcceleration (Math|Float|Power (Variables|Default|GetAcceleration) 1.2))
  (Variables|/Script/Engine.MovementComponent|SetVelocity (Variables|Default|GetProjectileMovement) (+ (* (Math|Vector|Normalize (Variables|/Script/Engine.MovementComponent|GetVelocity (Variables|Default|GetProjectileMovement))) (Variables|Default|GetAcceleration)) (Variables|/Script/Engine.MovementComponent|GetVelocity (Variables|Default|GetProjectileMovement)))))

(event Collision|EventActorBeginOverlap
  (params (OtherActor :type Actor%20Object%20Reference))
  (|CallParentFunction OtherActor) ; This node is disabled and will not be called.\nDrag off pins to build functionality.
)

(event EventTick
  (params (DeltaSeconds :type Float%20%28single-precision%29))
  (|CallParentFunction DeltaSeconds))

(event EventHit
  (params (MyComp :type Primitive%20Component%20Object%20Reference) (Other :type Actor%20Object%20Reference) (OtherComp :type Primitive%20Component%20Object%20Reference) (bSelfMoved :type Boolean) (HitLocation :type Vector :default "0, 0, 0") (HitNormal :type Vector :default "0, 0, 0") (NormalImpulse :type Vector :default "0, 0, 0") (Hit :type Hit%20Result%20Structure%20%28by%20ref%29))
  (|CallParentFunction MyComp Other OtherComp bSelfMoved HitLocation HitNormal NormalImpulse Hit)
  (Game|SpawnActorfromClass "/Game/Blueprints/Weapons/Projectiles/BP_Explosion.BP_Explosion_C" (Transformation|GetActorTransform) "Undefined" self 0)
  (Actor|DestroyActor))

(fn ConstructionScript
  (|CallParentFunction))

(fn OnEndonHit)

(fn SpawnDecal)

(fn AddPhysicsImpulse)