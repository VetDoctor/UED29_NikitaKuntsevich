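; Short-lived muzzle flash effect actor for weapons, pairing a mesh with a point light.
; On BeginPlay it randomizes the mesh's base scale, then a timeline curve drives both that scale and the light intensity, each multiplied by its own coefficient.
; A timer matching the timeline length is set alongside, apparently to call ReadyToDestroy, which destroys the actor.
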(event EventBeginPlay
  (Utilities|FlowControl|Sequence
    (:then_0
      (Variables|Default|SetMuzzleScale (CallFunction|RNGVector (Transformation|GetWorldScale (Variables|Default|GetMuzzleMesh)) 0.8 1.2))
      (bind _scalea (Timeline|MuzzleTimeline Play)
        (:Update
          (Transformation|SetWorldScale3D (Variables|Default|GetMuzzleMesh) (* (Variables|Default|GetMuzzleScale) (* (Variables|Default|GetMuzzleScaleCoef) _scalea)))
          (Rendering|Components|Light|SetIntensity (Variables|Default|GetPointLight) (* _scalea (Variables|Default|GetLightCoef))))))
    (:then_1
      (Utilities|Time|SetTimerbyEvent (EventDispatchers|CreateEvent :!event ReadytoDestroy) (Components|Timeline|GetTimelineLength (Variables|Default|GetMuzzleTimeline))))))

(event Collision|EventActorBeginOverlap
  (params (OtherActor :type Actor%20Object%20Reference)))

(event EventTick
  (params (DeltaSeconds :type Float%20%28single-precision%29)))

(fn ConstructionScript)

(fn ReadytoDestroy
  (Actor|DestroyActor))