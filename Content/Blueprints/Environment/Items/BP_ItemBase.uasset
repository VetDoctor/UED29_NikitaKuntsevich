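; Base item actor that shows a text prompt while a Character overlaps it and can be picked up into a backpack.
; Overlap stores the character and enables interaction; Tick turns the text toward the third-person character's root location, not the actual camera.
; Interacts passes the character's BP_BackpackComponent to PutIntoBackPack, an empty stub here, and returns true on every path.
; AfterUse destroys the item.
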(event EventBeginPlay
  (Rendering|SetVisibility (Variables|Default|GetTextRender) false false))

(event Collision|EventActorBeginOverlap
  (params (OtherActor :type Actor%20Object%20Reference))
  (bind _ascharacter (Utilities|Casting|CastToCharacter OtherActor))
  (Variables|Default|SetCharacterInBox _ascharacter)
  (Rendering|SetVisibility (Variables|Default|GetTextRender) true false)
  (Variables|Default|SetIsReadyToInteract true)
  (Variables|Default|SetIsLookingAtPlayerCamera true))

(event Collision|EventActorEndOverlap
  (params (OtherActor :type Actor%20Object%20Reference))
  (Utilities|Casting|CastToCharacter OtherActor)
  (Variables|Default|SetCharacterInBox 0)
  (Rendering|SetVisibility (Variables|Default|GetTextRender) false false)
  (Variables|Default|SetIsReadyToInteract false)
  (Variables|Default|SetIsLookingAtPlayerCamera false))

(event EventTick
  (params (DeltaSeconds :type Float%20%28single-precision%29))
  (CallFunction|LookingatPlayerCamera))

(fn ConstructionScript)

(fn LookingatPlayerCamera
  (if (Variables|Default|GetIsLookingAtPlayerCamera)
    (bind _characterinbox (Variables|Default|GetCharacterInBox)
      (:then
        (bind _asbp_third_person_character (Utilities|Casting|CastToBP_ThirdPersonCharacter _characterinbox))
        (LocalVariables|SetCameraLocation (Transformation|GetWorldLocation (Variables|/Script/Engine.Actor|GetRootComponent _asbp_third_person_character)))
        (Transformation|SetWorldRotation (Variables|Default|GetTextRender) (Math|Rotator|FindLookatRotation (Transformation|GetWorldLocation (Variables|Default|GetTextRender)) (LocalVariables|GetCameraLocation)) false false))
      (:else))))

(fn PutIntoBackPack
  (params (InBackpack :type BP%20Backpack%20Component%20Object%20Reference)))

(fn AfterUse
  (Actor|DestroyActor))

(fn Interacts
  (if (Variables|Default|GetIsReadyToInteract)
    (bind _characterinbox (Variables|Default|GetCharacterInBox)
      (:then
        (Utilities|IsValid (Actor|GetComponentbyClass _characterinbox "/Game/Blueprints/Components/BP_BackpackComponent.BP_BackpackComponent_C")
          (:Is%20Valid
            (CallFunction|PutIntoBackPack (Actor|GetComponentbyClass _characterinbox "/Game/Blueprints/Components/BP_BackpackComponent.BP_BackpackComponent_C"))
            (return true))
          (:Is%20Not%20Valid
            (return true))))
      (:else
        (return true)))
    (else
      (return true))))