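; Lockable door, extending a parent door, that opens or closes on interaction and shows its lock state with a red or green point light.
; When locked, Interacts searches the overlapping actor's backpack component for the required quest items and unlocks if all are found.
; Matching keys are removed as found, even if the set is incomplete.
; SwitchLock and Unlock change the state directly, while Lock only locks when no keys are listed.
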(event EventTick
  (params (DeltaSeconds :type Float%20%28single-precision%29))
  (|CallParentFunction DeltaSeconds) ; This node is disabled and will not be called.\nDrag off pins to build functionality.
)

(event EventCloseDoor
  (|CallParentFunction))

(event EventOpenDoor
  (if (not (Variables|DoorConfigure|GetIsDoorLocked))
    (|CallParentFunction)))

(fn ConstructionScript
  (|CallParentFunction)
  (CallFunction|UpdateDoorLockIndication))

(fn SwitchLock
  (Variables|DoorConfigure|SetIsDoorLocked (not (Variables|DoorConfigure|GetIsDoorLocked)))
  (CallFunction|UpdateDoorLockIndication))

(fn UpdateDoorLockIndication
  (Rendering|Components|Light|SetLightColor (Variables|Default|GetPointLightLockIndicator) (Math|Color|SelectColor "(R=0.932292,G=0.000000,B=0.000000,A=1.000000)" "(R=0.000000,G=0.359375,B=0.042627,A=1.000000)" (Variables|DoorConfigure|GetIsDoorLocked)) true))

(fn Lock
  (if true
    (Variables|DoorConfigure|SetIsDoorLocked (not (Utilities|Array|IsValidIndex (Variables|Default|GetNeededKeysName))))
    (CallFunction|UpdateDoorLockIndication)))

(fn Unlock
  (Variables|DoorConfigure|SetIsDoorLocked false)
  (CallFunction|UpdateDoorLockIndication))

(fn Interacts
  (if (Variables|Default|GetIsReadyToInteract)
    (if (not (Variables|DoorConfigure|GetIsDoorLocked))
      (if (Variables|Default|GetIsDoorOpen)
        (CallFunction|CloseDoor)
        (return true)
        (else
          (CallFunction|OpenDoor)
          (return true)))
      (elif (Utilities|Array|IsValidIndex (Variables|Default|GetNeededKeysName))
        (bind _overlappedactor (Variables|Default|GetOverlappedActor)
          (:then
            (Utilities|IsValid (Actor|GetComponentbyClass _overlappedactor "/Game/Blueprints/Components/BP_BackpackComponent.BP_BackpackComponent_C")
              (:Is%20Valid
                (LocalVariables|SetL_BackPack (Actor|GetComponentbyClass _overlappedactor "/Game/Blueprints/Components/BP_BackpackComponent.BP_BackpackComponent_C"))
                (for _array_element (Variables|Default|GetNeededKeysName)
                  (LocalVariables|SetL_ItemName _array_element)
                  (if (Utilities|Set|Contains (Variables|/Game/Blueprints/Components/BP_BackpackComponent.BP_BackpackComponent_C|GetQuestItems (LocalVariables|GetL_BackPack)) (LocalVariables|GetL_ItemName))
                    (Math|Integer|IncrementInt (LocalVariables|GetL_ItemInriment)
                      (:%20%20
                        ;[0.2139 0.1473 1] If you want to remove item
                        (Default|RemoveQuestItem (LocalVariables|GetL_BackPack) (LocalVariables|GetL_ItemName))))))
                (if (== (LocalVariables|GetL_ItemInriment) (Utilities|Array|Length (Variables|Default|GetNeededKeysName)))
                  (CallFunction|Unlock)
                  (else
                    (return true))))
              (:Is%20Not%20Valid
                (return true))))
          (:else
            (return true)))
        (else
          (return true))))
    (else
      (return false))))